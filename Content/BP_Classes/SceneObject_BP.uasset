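; Puzzle scene object that the player manipulates with the mouse until it matches a target position and rotation.
; Hover drives a material highlight and sound; clicking starts manipulation until Pawn_BP reports mouse release.
; Each Tick applies Pawn_BP mouse input as yaw, Ctrl-held roll or Shift-held swept movement, the latter two optional.
; A delayed check compares the transform against tolerances, then marks it valid, stopping Tick and hover feedback.
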(event OnBeginCursorOver(StaticMeshComponent)
  (params (TouchedComponent :type Primitive%20Component%20Object%20Reference))
  (if (not (Variables|Default|GetDisable))
    (if (Variables|Input|GetLeftClick)
      _
      (else
        (Audio|PlaySound2D "/Game/Sounds/Effects/mixkit-small-hit-in-a-game-2072.mixkit-small-hit-in-a-game-2072" 1.0 1.0 0.0 0 0)))
    (Rendering|Material|SetScalarParameterValueonMaterials (Variables|Default|GetStaticMeshComponent) "HighLightONOFF" 1e+01)))

(event OnEndCursorOver(StaticMeshComponent)
  (params (TouchedComponent :type Primitive%20Component%20Object%20Reference))
  (if (not (Variables|Input|GetLeftClick))
    (Rendering|Material|SetScalarParameterValueonMaterials (Variables|Default|GetStaticMeshComponent) "HighLightONOFF" 0.0)))

(event OnClicked(StaticMeshComponent)
  (params (TouchedComponent :type Primitive%20Component%20Object%20Reference) (ButtonPressed :type Key%20Structure :default "None"))
  (Variables|Input|SetLeftClick true)
  (Utilities|FlowControl|DoOnce true) ; enters at Reset
)

(event Custom|On%20Mouse%20Released%20Secure
  (Utilities|FlowControl|DoOnce true
    (:Completed
      (Variables|Input|SetLeftClick false)
      (if (not (Variables|/Game/BP_Classes/GameLoop/Pawn_BP.Pawn_BP_C|GetStilOverlap? (Variables|Default|GetPawnBP)))
        (Rendering|Material|SetScalarParameterValueonMaterials (Variables|Default|GetStaticMeshComponent) "HighLightONOFF" 0.0)))))

(event EventBeginPlay
  (bind _aspawn_bp (Utilities|Casting|CastToPawn_BP (Game|Player|GetPlayerPawn 0) :!label _label)
    (:then
      (Variables|Default|SetPawnBP _aspawn_bp))
    (:CastFailed
      (Utilities|FlowControl|Delay 0.1)
      (goto _label))))

(event EventTick
  (params (DeltaSeconds :type Float%20%28single-precision%29))
  (bind _pawnbp (Variables|Default|GetPawnBP))
  (if (Variables|Validation|GetValid)
    (Actor|Tick|SetActorTickEnabled false)
    (Variables|Default|SetDisable true)
    (elif (Variables|Input|GetLeftClick)
      (Utilities|ObjectValidation
        (:Exit
          (if (Variables|/Game/BP_Classes/GameLoop/Pawn_BP.Pawn_BP_C|GetMouseReleased? _pawnbp)
            (CallFunction|OnMouseReleasedSecure))
          (if (Variables|/Game/BP_Classes/GameLoop/Pawn_BP.Pawn_BP_C|GetLeftCtrl_Pressed? _pawnbp)
            (Utilities|RollRotation)
            (elif (Variables|/Game/BP_Classes/GameLoop/Pawn_BP.Pawn_BP_C|GetLeftShift_Pressed? _pawnbp)
              (Utilities|Movement)
              (else
                (Utilities|YawRotation)))))))))

(fn ConstructionScript)