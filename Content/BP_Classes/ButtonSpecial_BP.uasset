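; Clickable 3D menu button whose MenuTypeName selects its action: open the level of that name, quit, reset the save, toggle window mode or toggle audio.
; Clicking plays a sound, sinks Base and raises LoadLevel, while release lifts Base and clears the flag.
; A delayed Tick polls LoadLevel to run the action.
; Audio and resolution state live in GameInstance_BP, applied through sound mix overrides and GameUserSettings.
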(event OnClicked(Base)
  (params (TouchedComponent :type Primitive%20Component%20Object%20Reference) (ButtonPressed :type Key%20Structure :default "None"))
  (Audio|PlaySound2D "/Game/Sounds/Effects/mixkit-neutral-bot-pinbal-tone-3137.mixkit-neutral-bot-pinbal-tone-3137" 1.0 1.0 0.0 0 0)
  (Transformation|AddLocalOffset (Variables|Default|GetBase) "0, 0,-10.000000" false false)
  (Variables|Default|SetLoadLevel true)
  (Variables|Default|SetClicked? true))

(event OnReleased(Base)
  (params (TouchedComponent :type Primitive%20Component%20Object%20Reference) (ButtonReleased :type Key%20Structure :default "None"))
  (Development|PrintString "Released")
  (if (Variables|Default|GetClicked?)
    (Transformation|AddLocalOffset (Variables|Default|GetBase) "0,0.000000,10.000000" false false)
    (Variables|Default|SetLoadLevel false)
    (Variables|Default|SetClicked? false)))

(event EventBeginPlay
  (bind _asgame_instance_bp (Utilities|Casting|CastToGameInstance_BP (Game|GetGameInstance)))
  (Variables|Default|SetGameInstancerBP _asgame_instance_bp))

(event EventTick
  (params (DeltaSeconds :type Float%20%28single-precision%29))
  (bind _gameinstancerbp (Variables|Default|GetGameInstancerBP))
  (Utilities|FlowControl|Delay 0.05)
  (if (Variables|Default|GetLoadLevel)
    (Variables|Default|SetLoadLevel false)
    (Utilities|FlowControl|Delay 0.3)
    (switch name (Variables|Default|GetMenuTypeName)
      (:Default
        (Game|OpenLevel(byName) (Variables|Default|GetMenuTypeName)))
      (:Exit
        (Game|QuitGame 0 "Quit" false))
      (:Reset
        (SaveGame|DeleteGameinSlot "Save00")
        (Development|PrintString "DeleteSaveGame")
        (Game|OpenLevel(byName) "Menu"))
      (:Window
        (Utilities|SetResolution))
      (:Audio
        (Variables|/Game/BP_Classes/GameLoop/GameInstance_BP.GameInstance_BP_C|SetAudio? _gameinstancerbp (not (Variables|/Game/BP_Classes/GameLoop/GameInstance_BP.GameInstance_BP_C|GetAudio? _gameinstancerbp)))
        (if (Variables|/Game/BP_Classes/GameLoop/GameInstance_BP.GameInstance_BP_C|GetAudio? (Variables|Default|GetGameInstancerBP))
          (Development|PrintString "Audio ON")
          (Audio|SetSoundMixClassOverride "/Game/Sounds/MusicMix.MusicMix" "/Engine/EngineSounds/Music.Music" 1.0 1.0 1.0 true)
          (Audio|PushSoundMixModifier "/Game/Sounds/MusicMix.MusicMix")
          (Audio|SetSoundMixClassOverride "/Game/Sounds/EffectMix.EffectMix" "/Engine/EngineSounds/SFX.SFX" 1.0 1.0 1.0 true)
          (Audio|PushSoundMixModifier "/Game/Sounds/EffectMix.EffectMix")
          (else
            (Development|PrintString "Audio OFF")
            (Audio|SetSoundMixClassOverride "/Game/Sounds/MusicMix.MusicMix" "/Engine/EngineSounds/Music.Music" 0.0 1.0 1.0 true)
            (Audio|PushSoundMixModifier "/Game/Sounds/MusicMix.MusicMix")
            (Audio|SetSoundMixClassOverride "/Game/Sounds/EffectMix.EffectMix" "/Engine/EngineSounds/SFX.SFX" 0.0 1.0 1.0 true)
            (Audio|PushSoundMixModifier "/Game/Sounds/EffectMix.EffectMix")))))))

(fn ConstructionScript)