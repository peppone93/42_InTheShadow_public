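; Game mode for InTheShadow that sets up display resolution on BeginPlay when the GameInstance_BP Start flag is set.
; It stores the middle entry of the supported fullscreen resolutions as the windowed resolution and a fixed 1080p as the fullscreen one in the game instance.
; It then applies a hardcoded 720p windowed mode through GameUserSettings, independent of those stored values.
; The Start flag is only read here, never cleared.
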(event EventBeginPlay
  (bind _asgame_instance_bp (Utilities|Casting|CastToGameInstance_BP (Game|GetGameInstance))
    (:then
      (if (Variables|/Game/BP_Classes/GameLoop/GameInstance_BP.GameInstance_BP_C|GetStart _asgame_instance_bp)
        (Utilities|FlowControl|Sequence
          (:then_0
            (bind _resolutions (Class|KismetSystemLibrary|GetSupportedFullscreenResolutions))
            (bind _asgame_instance_bp_2 (Utilities|Casting|CastToGameInstance_BP (Game|GetGameInstance)))
            (Variables|/Game/BP_Classes/GameLoop/GameInstance_BP.GameInstance_BP_C|SetWinRes _asgame_instance_bp_2 (Utilities|Array|Get(acopy) _resolutions (/ (Utilities|Array|Length _resolutions) 2)))
            (Variables|/Game/BP_Classes/GameLoop/GameInstance_BP.GameInstance_BP_C|SetFullRes _asgame_instance_bp_2 (Utilities|Struct|MakeIntPoint 1920 1080)))
          (:then_1
            (bind _returnvalue (Settings|GetGameUserSettings))
            (Class|GameUserSettings|SetScreenResolution _returnvalue (Utilities|Struct|MakeIntPoint 1280 720))
            (Class|GameUserSettings|SetFullscreenMode _returnvalue "Windowed")
            (Class|GameUserSettings|ApplyResolutionSettings _returnvalue false)
            (Class|GameUserSettings|ApplySettings _returnvalue true)))))
    (:CastFailed
      (Development|PrintString "GameInstanceCastFail"))))

(fn ConstructionScript)