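; Player pawn that holds input state for mouse-driven interaction with scene objects.
; On BeginPlay it optionally applies manual camera exposure and caches the PlayerController_BP reference, printing whether the cast succeeded.
; Mouse axes, Ctrl, Shift and left-button state are stored in variables.
; On left-button release, a cursor trace records whether a SceneObject_BP is still underneath, a workaround for checking overlap outside the object's Blueprint.
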(event EventBeginPlay
  (if (!= (Variables|Rendering|GetExposure) -1)
    (Utilities|Struct|SetmembersinPostProcessSettings (Variables|/Script/Engine.CameraComponent|GetPostProcessSettings (Variables|Default|GetCamera)) "AEM_Manual" (Math|Conversions|ToFloat(Integer) (Variables|Rendering|GetExposure))))
  (bind _asplayer_controller_bp (Utilities|Casting|CastToPlayerController_BP (Game|GetPlayerController 0))
    (:then
      (Variables|Default|SetPlayerController _asplayer_controller_bp)
      (Development|PrintString "Set"))
    (:CastFailed
      (Development|PrintString "Fail"))))

(event Collision|EventActorBeginOverlap
  (params (OtherActor :type Actor%20Object%20Reference)))

(event Input|MouseEvents|MouseX
  (params (AxisValue :type Float%20%28single-precision%29))
  (Variables|Default|SetMouseX AxisValue))

(event Input|MouseEvents|MouseY
  (params (AxisValue :type Float%20%28single-precision%29))
  (Variables|Default|SetMouseY AxisValue))

(event Input|KeyboardEvents|LeftCtrl
  (params (Key :type Key%20Structure :default "None"))
  (:Pressed
    (Variables|Default|SetLeftCtrl_Pressed? true))
  (:Released
    (Variables|Default|SetLeftCtrl_Pressed? false)))

(event Input|KeyboardEvents|LeftShift
  (params (Key :type Key%20Structure :default "None"))
  (:Pressed
    (Variables|Default|SetLeftShift_Pressed? true))
  (:Released
    (Variables|Default|SetLeftShift_Pressed? false)))

(event Input|MouseEvents|LeftMouseButton
  (params (Key :type Key%20Structure :default "None"))
  (:Pressed
    (Variables|Default|SetMouseReleased? false))
  (:Released
    (Variables|Default|SetMouseReleased? true)
    ;[1 1 1] TrickToCheckOverlap Out of Oject BP
    (Utilities|Casting|CastToSceneObject_BP (.HitActor (Collision|BreakHitResult (.HitResult (Game|Player|GetHitResultUnderCursorbyChannel (Game|GetPlayerController 0) "TraceTypeQuery1" true))))
      (:then
        (Variables|Default|SetStilOverlap? true))
      (:CastFailed
        (Variables|Default|SetStilOverlap? false)))))

(fn ConstructionScript)