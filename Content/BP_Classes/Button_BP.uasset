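; Clickable 3D button actor that opens the level named in its LevelName variable once activated.
; ActiveButton and DeactivateButton toggle the light, material highlight and Activated flag.
; Clicking plays a sound and, when active, sinks the base and sets LoadLevel, which release reverses.
; Tick runs the Flink macro, ping-ponging the Connection material highlight through delays while active, then opens the level if LoadLevel is set.
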(event OnClicked(Base)
  (params (TouchedComponent :type Primitive%20Component%20Object%20Reference) (ButtonPressed :type Key%20Structure :default "None"))
  (Audio|PlaySound2D "/Game/Sounds/Effects/mixkit-neutral-bot-pinbal-tone-3137.mixkit-neutral-bot-pinbal-tone-3137" 1.0 1.0 0.0 0 0)
  (if (Variables|Default|GetActivated?)
    (Transformation|AddLocalOffset (Variables|Default|GetBase) "0, 0,-15.000000" false false)
    (Variables|Level|SetLoadLevel? true)))

(event OnReleased(Base)
  (params (TouchedComponent :type Primitive%20Component%20Object%20Reference) (ButtonReleased :type Key%20Structure :default "None"))
  (if (Variables|Default|GetActivated?)
    (Transformation|AddLocalOffset (Variables|Default|GetBase) "0,0.000000,15.000000" false false)
    (Variables|Level|SetLoadLevel? false)))

(event EventBeginPlay
  (bind _asgame_instance_bp (Utilities|Casting|CastToGameInstance_BP (Game|GetGameInstance)))
  (Variables|Default|SetGameInstance _asgame_instance_bp))

(event Collision|EventActorBeginOverlap
  (params (OtherActor :type Actor%20Object%20Reference)))

(event EventTick
  (params (DeltaSeconds :type Float%20%28single-precision%29))
  (Utilities|FlowControl|Delay 0.05)
  (Utilities|Flink
    (:Exit
      (if (Variables|Level|GetLoadLevel?)
        (Variables|Level|SetLoadLevel? false)
        (Utilities|FlowControl|Delay 0.3)
        (Game|OpenLevel(byName) (Utilities|String|StringToName (Variables|Level|GetLevelName)))))))

(fn ConstructionScript)

(fn ActiveButton
  (Rendering|Components|Light|SetIntensity (Variables|Default|GetLight) 5.4e+03)
  (Rendering|Material|SetScalarParameterValueonMaterials (Variables|Default|GetBase) "HighLightONOFF" 1.0)
  (Variables|Default|SetActivated? true)
  (return))

(fn DeactivateButton
  (Rendering|Components|Light|SetIntensity (Variables|Default|GetLight) 0.0)
  (Rendering|Material|SetScalarParameterValueonMaterials (Variables|Default|GetBase) "HighLightONOFF" 0.0)
  (Variables|Default|SetActivated? false)
  (return))